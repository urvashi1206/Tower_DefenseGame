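; Anim notify that triggers a combat area-of-effect hit, named for a howl animation marker.
; On notify it finds the mesh owner's BP_CombatComponent and, if valid, calls GenerateAreaOfEffect at the hit socket's location.
; Radius, damage, status effect and debug mode come from the notify's own variables, and the component handles the hit itself.
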(fn ReceivedNotify
  (params (MeshComp :type Skeletal%20Mesh%20Component%20Object%20Reference) (Animation :type Anim%20Sequence%20Base%20Object%20Reference) (EventReference :type Anim%20Notify%20Event%20Reference%20Structure%20%28by%20ref%29))
  (bind _returnvalue (Components|GetOwner MeshComp))
  (bind _returnvalue_2 (Actor|GetComponentbyClass _returnvalue "/Game/Blueprints/AI/Components/BP_CombatComponent.BP_CombatComponent_C"))
  ;[1 1 1] Take in notify parameters and generate a hit sphere or area of effect
  (Utilities|IsValid _returnvalue_2
    (:Is%20Valid
      (Default|GenerateAreaOfEffect _returnvalue_2 (Transformation|GetSocketLocation MeshComp (Variables|Default|GetHitSocket)) (Variables|Default|GetRadius) (Variables|Default|GetDamage) (Variables|Default|GetDebug%20Mode) (Variables|Default|GetStatus%20Effect))
      (return true))))