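; BP_EnemyManager runs night waves of werewolves, driven by the BP_TimeManager day/night change event.
; On BeginPlay it caches every existing BP_Werewolf and BP_EnemySpawn, treating the werewolves as a pool rather than spawning new actors.
; At night it teleports out-of-combat werewolves to random spawn points and flags them InCombat.
; At day it resets in-combat ones by dealing max-health damage, then increases the wave size.
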(event Custom|HandleTimeCycle
  (params (bIsDay :type Boolean))
  ;[1 1 1] Bind Day Shift Delegate for enemy management logic
  (if bIsDay
    ;[1 1 1] Update Wave Parameters and reset enemies in combat
    (CallFunction|ResetEnemies)
    (CallFunction|UpdateWaveParameters)
    (else
      ;[1 1 1] Spawn next wave of enemies
      (CallFunction|SpawnEnemies (Variables|Default|GetWaveSize)))))

(event EventBeginPlay
  ;[1 1 1] Init all actor arrays
  (bind _outactors (Actor|GetAllActorsOfClass "/Game/Blueprints/AI/Characters/BP_Werewolf.BP_Werewolf_C"))
  (Variables|Default|SetEnemies _outactors)
  (bind _outactors_2 (Actor|GetAllActorsOfClass "/Game/Blueprints/AI/Management/BP_EnemySpawn.BP_EnemySpawn_C"))
  (Variables|Default|SetSpawnPoints _outactors_2)
  (bind _returnvalue (Actor|GetActorOfClass "/Game/Blueprints/BP_TimeManager.BP_TimeManager_C"))
  ;[1 1 1] Bind Day Shift Delegate for enemy management logic
  (EventDispatchers|AssignChangeOfTime _returnvalue (delegate Custom|HandleTimeCycle)))

(fn ConstructionScript)

(fn SpawnEnemies
  (params (Enemy%20Count :type Integer))
  ;[1 1 1] Loop through desired enemy count and spawn enemies
  (for _index (range 0 Enemy%20Count)
    (CallFunction|SpawnEnemy)))

(fn GetNextAvailableEnemy
  ;[1 1 1] Iterate through all enemies until you find one not in combat
  (for _array_element (Variables|Default|GetEnemies)
    (if (not (Variables|/Game/Blueprints/AI/Characters/BP_Werewolf.BP_Werewolf_C|GetInCombat _array_element))
      (return _array_element))))

(fn SpawnEnemy
  ;[1 1 1] Get the next available enemy, update location and combat status
  (bind _enemy (CallFunction|GetNextAvailableEnemy))
  (Utilities|IsValid _enemy
    (:Is%20Valid
      (LocalVariables|SetSpawnedEnemy _enemy)
      (Transformation|SetActorLocation (LocalVariables|GetSpawnedEnemy) (Transformation|GetActorLocation (.OutItem (Utilities|Array|Random (Variables|Default|GetSpawnPoints)))) false false)
      (Variables|/Game/Blueprints/AI/Characters/BP_Werewolf.BP_Werewolf_C|SetInCombat (LocalVariables|GetSpawnedEnemy) true))))

(fn ResetEnemies
  ;[1 1 1] Iterate through each enemy in combat and reset them by dealing max damage
  (bind _enemiesincombat (CallFunction|GetAllEnemiesinCombat))
  (for _array_element _enemiesincombat
    (Default|TakeDamage (Variables|/Game/Blueprints/AI/Characters/BP_Werewolf.BP_Werewolf_C|GetBP_CombatComponent _array_element) (Variables|/Game/Blueprints/AI/Components/BP_CombatComponent.BP_CombatComponent_C|GetMaxHealth (Variables|/Game/Blueprints/AI/Characters/BP_Werewolf.BP_Werewolf_C|GetBP_CombatComponent _array_element)))))

(fn GetAllEnemiesinCombat
  ;[1 1 1] Iterate through all enemies and return any in combat
  (for _array_element (Variables|Default|GetEnemies)
    (if (Variables|/Game/Blueprints/AI/Characters/BP_Werewolf.BP_Werewolf_C|GetInCombat _array_element)
      (Utilities|Array|AddUnique (LocalVariables|GetInCombatArray) _array_element)))
  (return (LocalVariables|GetInCombatArray)))

(fn UpdateWaveParameters
  ;[1 1 1] Increase Wave Size
  (Variables|Default|SetWaveSize (+ (Variables|Default|GetWaveSize) (Variables|Default|GetWaveIncrement))))