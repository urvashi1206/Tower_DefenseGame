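; AI controller for enemies that runs BT_EnemyBT on BeginPlay and alerts it to sensed build structures.
; When AI perception senses a BP_BuildActor, it writes the TargetLocation blackboard key and sets StructDetected to true.
; An unsuccessful stimulus from any actor clears StructDetected, while TargetLocation keeps its last value.
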(event OnTargetPerceptionUpdated(AIPerception)
  (params (Actor :type Actor%20Object%20Reference) (Stimulus :type AI%20Stimulus%20Structure))
  (if (.bsuccessfullysensed Stimulus)
    ;[1 1 1] If a struct is detected then set its location as enemy's target and then set detected struct to true
    (Utilities|Casting|CastToBP_BuildActor Actor)
    (AI|Components|Blackboard|SetValueasVector (AI|GetBlackboard 0) (Utilities|Name|MakeLiteralName "TargetLocation") (Transformation|GetActorLocation))
    (AI|Components|Blackboard|SetValueasBool (AI|GetBlackboard 0) (Utilities|Name|MakeLiteralName "StructDetected") true)
    (else
      ;[1 1 1] If no actors are perceived then clear blackboard key
      (AI|Components|Blackboard|ClearValue (AI|GetBlackboard 0) (Utilities|Name|MakeLiteralName "StructDetected")))))

(event EventBeginPlay
  ;[1 1 1] At start, the controller will run the enemy's behavior tree
  (AI|RunBehaviorTree "/Game/Blueprints/AI/TreesAndBoards/BT_EnemyBT.BT_EnemyBT"))

(fn ConstructionScript)