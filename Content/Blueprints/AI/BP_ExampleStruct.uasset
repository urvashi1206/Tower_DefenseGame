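; BP_ExampleStruct is an actor that displays a health bar through a widget component.
; On BeginPlay it casts the component's widget to BP_Healthbar and sets the actor as its OwningActor.
; Every Tick it billboards the widget toward player 0's camera, computing yaw with Atan2 so it turns only around the vertical axis.
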(event EventBeginPlay
  ;[1 1 1] Initialize owning actor of health bar widget to be this actor
  (bind _asbp_healthbar (Utilities|Casting|CastToBP_Healthbar (UserInterface|GetWidget (Variables|Default|GetWidget))))
  (Variables|/Game/Blueprints/AI/BP_Healthbar.BP_Healthbar_C|SetOwningActor _asbp_healthbar (Components|GetOwner (Variables|Default|GetDefaultSceneRoot))))

(event EventTick
  (params (DeltaSeconds :type Float%20%28single-precision%29))
  (bind _returnvalue (Game|GetPlayerCameraManager 0))
  (bind _widget (Variables|Default|GetWidget))
  (bind _returnvalue_2 (Camera|GetCameraLocation _returnvalue))
  (bind _returnvalue_3 (Transformation|GetWorldLocation _widget))
  (Transformation|SetWorldRotation (Variables|Default|GetWidget) (Math|Vector|RotatorfromAxisandAngle "0.000000,0.000000,1.000000" (Class|KismetMathLibrary|DegAtan2 (- (.y _returnvalue_2) (.y _returnvalue_3)) (- (.x _returnvalue_2) (.x _returnvalue_3)))) false false))

(fn ConstructionScript)