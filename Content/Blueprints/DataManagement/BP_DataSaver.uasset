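; BP_DataSaver records end-of-play statistics for a play-through and writes them to disk.
; SaveData reads days survived from BP_TimeManager and counts placed Wall, LumberMill and Outpost actors in the level.
; It combines these with tracked totals for sugar, spending, repairs, upgrades, destruction and kills into a SaveData struct.
; The struct is written as a JSON file named with a fresh UUID under the project file path.
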(fn ConstructionScript)

(fn SaveData
  (Utilities|FlowControl|Sequence
    (:then_0
      ;[1 1 1] Get all gameplay data stored throughout play-through and set the struct in preparation for file saving
      (bind _returnvalue (Actor|GetActorOfClass "/Game/Blueprints/BP_TimeManager.BP_TimeManager_C"))
      (LocalVariables|SetDaysSurvived (Math|Float|Truncate (Variables|/Game/Blueprints/BP_TimeManager.BP_TimeManager_C|GetDayCounter _returnvalue)))
      (bind _outactors (Actor|GetAllActorsOfClass "/Game/Maps/Blueprints/Wall.Wall_C"))
      (LocalVariables|SetWallsPlaced (Utilities|Array|Length _outactors))
      (bind _outactors_2 (Actor|GetAllActorsOfClass "/Game/Maps/Blueprints/LUmberMIll.LUmberMIll_C"))
      (LocalVariables|SetMillsPlaced (Utilities|Array|Length _outactors_2))
      (bind _outactors_3 (Actor|GetAllActorsOfClass "/Game/Maps/Blueprints/Outpost.Outpost_C"))
      (LocalVariables|SetOutpostsPlaced (Utilities|Array|Length _outactors_3))
      (LocalVariables|SetDataToSave (Utilities|Struct|MakeSaveData (LocalVariables|GetDaysSurvived) (LocalVariables|GetWallsPlaced) (LocalVariables|GetMillsPlaced) (LocalVariables|GetOutpostsPlaced) (Variables|Default|GetTotalSugar) (Variables|Default|GetTotalMoneySpent) (Variables|Default|GetTotalRepairs) (Variables|Default|GetTotalUpgrades) (Variables|Default|GetTotalDestroyed) (Variables|Default|GetTotalEnemiesKilled))))
    (:then_1
      ;[1 1 1] Save data to file in JSON format
      (bind _returnvalue_2 (Class|DataManager|GenerateUUID))
      (Class|DataManager|WriteSaveDatatoJsonFile (Utilities|String|Append (Utilities|String|Append (Class|BlueprintPathsLibrary|GetProjectFilePath) _returnvalue_2) ".json") (LocalVariables|GetDataToSave)))))