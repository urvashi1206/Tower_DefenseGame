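; Outpost actor with a mesh and a detection sphere that finds the closest werewolf enemy.
; Sphere overlap compares the overlapped component to BP_Werewolf, and on a match sets a found flag, prints a debug message and calls Attack.
; Attack scans every BP_Werewolf in the level by distance to the mesh and stores the nearest as ClosestEnemy; it applies no damage or other action.
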(event OnComponentBeginOverlap(Sphere)
  (params (OverlappedComponent :type Primitive%20Component%20Object%20Reference) (OtherActor :type Actor%20Object%20Reference) (OtherComp :type Primitive%20Component%20Object%20Reference) (OtherBodyIndex :type Integer) (bFromSweep :type Boolean) (SweepResult :type Hit%20Result%20Structure%20%28by%20ref%29))
  (if (== OverlappedComponent "/Game/Blueprints/AI/Characters/BP_Werewolf.BP_Werewolf")
    (bind _output_get (Variables|Default|SetFIndEnemy? true))
    (Development|PrintString "find Enemy" _output_get)
    (CallFunction|Attack)))

(event Custom|Attack
  (bind _mesh (Variables|Character|GetMesh))
  (bind _returnvalue (Transformation|GetWorldLocation _mesh))
  (if (Variables|Default|GetFIndEnemy?)
    (bind _outactors (Actor|GetAllActorsOfClass "/Game/Blueprints/AI/Characters/BP_Werewolf.BP_Werewolf_C"))
    (Variables|Default|SetClosestEnemy (Utilities|Array|Get(acopy) _outactors))
    (for _array_element _outactors
      (if (< (Math|Vector|Distance(Vector) (Transformation|GetActorLocation _array_element) _returnvalue) (Math|Vector|Distance(Vector) _returnvalue (Transformation|GetActorLocation (Variables|Default|GetClosestEnemy))))
        (Variables|Default|SetClosestEnemy _array_element)))))

(event EventBeginPlay
  (|CallParentFunction) ; This node is disabled and will not be called.\nDrag off pins to build functionality.
)

(event Collision|EventActorBeginOverlap
  (params (OtherActor :type Actor%20Object%20Reference))
  (|CallParentFunction OtherActor) ; This node is disabled and will not be called.\nDrag off pins to build functionality.
)

(event EventTick
  (params (DeltaSeconds :type Float%20%28single-precision%29))
  (|CallParentFunction DeltaSeconds) ; This node is disabled and will not be called.\nDrag off pins to build functionality.
)

(fn ConstructionScript
  (|CallParentFunction))