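; Lumber mill actor that passively produces wood for the player each time day begins.
; On BeginPlay it finds the BP_TimeManager in the level and binds OnDayChange to its change-of-time event.
; When the change is to day, it spawns a PS_Woods effect at its location and adds a fixed amount to TotalWood on the player character's resource component.
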(event Custom|OnDayChange
  (params (bIsDay :type Boolean))
  (bind _bp_playercharacter (Variables|Default|GetBP_PlayerCharacter))
  (bind _bp_resourcecomponent (Variables|/Game/Maps/Blueprints/BP_Character.BP_Character_C|GetBP_ResourceComponent _bp_playercharacter))
  (if bIsDay
    (Niagara|SpawnSystematLocation "/Game/Maps/ParticleSystems/PS_Woods.PS_Woods" (Transformation|GetActorLocation))
    (Variables|/Game/Maps/Blueprints/BP_ResourceComponent.BP_ResourceComponent_C|SetTotalWood _bp_resourcecomponent (+ (Variables|/Game/Maps/Blueprints/BP_ResourceComponent.BP_ResourceComponent_C|GetTotalWood _bp_resourcecomponent) 20))))

(event EventBeginPlay
  (|CallParentFunction)
  (bind _returnvalue (Actor|GetActorOfClass "/Game/Blueprints/BP_TimeManager.BP_TimeManager_C"))
  (bind _output_get (Variables|Default|SetBP_TimeManager _returnvalue))
  (EventDispatchers|BindEventtoChangeOfTime _output_get (delegate Custom|OnDayChange)))

(event Collision|EventActorBeginOverlap
  (params (OtherActor :type Actor%20Object%20Reference))
  (|CallParentFunction OtherActor) ; This node is disabled and will not be called.\nDrag off pins to build functionality.
)

(fn ConstructionScript
  (|CallParentFunction))