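; BP_ResourceComponent is a resource component that handles spending from stored wood and sugar totals.
; WoodCollection and Sugar each subtract a given cost from their total and return true, or return false when the total is too low.
; Cookies follows the same check-and-deduct pattern but draws on TotalWood rather than a separate cookie total.
; BeginPlay and Tick are empty.
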(event EventBeginPlay)

(event EventTick
  (params (DeltaSeconds :type Float%20%28single-precision%29)))

(fn WoodCollection
  (params (WoodCost :type Integer))
  (if (>= (- (Variables|Default|GetTotalWood) WoodCost) 0)
    (Variables|Default|SetTotalWood (- (Variables|Default|GetTotalWood) WoodCost))
    (return true)
    (else
      (return false))))

(fn Sugar
  (params (SugarCost :type Integer))
  (if (>= (- (Variables|Default|GetTotalSugar) SugarCost) 0)
    (Variables|Default|SetTotalSugar (- (Variables|Default|GetTotalSugar) SugarCost))
    (return true)
    (else
      (return false))))

(fn Cookies
  (params (CookiesCost :type Integer))
  (if (>= (- (Variables|Default|GetTotalWood) CookiesCost) 0)
    (Variables|Default|SetTotalWood (- (Variables|Default|GetTotalWood) CookiesCost))
    (return true)
    (else
      (return false))))